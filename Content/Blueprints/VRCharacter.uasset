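; Player VR character with motion-controller grabbing and a mouse-and-keyboard fallback when no headset is enabled.
; Tick moves it relative to the left controller's flattened forward; without a headset, both controllers attach to the camera and movement uses ZQSD.
; Grips or triggers grab the first overlapped VRGripInterface actor or its gripping owner, hiding the hand and taking it from the other; release drops it.
; Pressing C possesses the last BikePawn found.
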(event `self.ReceiveBeginPlay`
  (bind _rightmotioncontroller (`self.RightMotionController`))
  (bind _leftmotioncontroller (`self.LeftMotionController`))
  (bind _vrreplicatedcamera (`self.VRReplicatedCamera`))
  (`|ExecutionSequence`
    (:`then_0`
      (if (`HeadMountedDisplayFunctionLibrary.IsHeadMountedDisplayEnabled`)
        (`HeadMountedDisplayFunctionLibrary.SetTrackingOrigin` "Floor")
        (else
          (`SceneComponent.K2_SetRelativeLocation` _vrreplicatedcamera (0.0 0.0 170.0) false false)
          (`SceneComponent.K2_SetRelativeLocation` _leftmotioncontroller (100.0 -40.0 20.0) false false)
          (`SceneComponent.K2_AttachToComponent` _leftmotioncontroller _vrreplicatedcamera "None" "KeepRelative" "KeepRelative" "KeepRelative" true)
          (`SceneComponent.K2_SetRelativeLocation` _rightmotioncontroller (60.0 40.0 -10.0) false false)
          (`SceneComponent.K2_AttachToComponent` _rightmotioncontroller _vrreplicatedcamera "None" "KeepRelative" "KeepRelative" "KeepRelative" true))))
    (:`then_1`
      ;[0.04384 0.4005 0.526] Movement
      (if (not (`HeadMountedDisplayFunctionLibrary.IsHeadMountedDisplayEnabled`))
        (set `CameraComponent.bUsePawnControlRotation` true (`self.VRReplicatedCamera`))))))

(event `Key|C`
  (params (Key :type "Key Structure"))
  (:`Pressed`
    (bind _outactors (`GameplayStatics.GetAllActorsOfClass` "/Game/Blueprints/BikePawn.BikePawn_C"))
    (bind _returnvalue (`KismetArrayLibrary.Array_LastIndex` _outactors))
    (if (>= _returnvalue 0)
      (`Controller.Possess` (`self.GetController`) (`|GetArrayItem` _outactors _returnvalue)))))

(event `Key|MouseScrollDown`
  (params (Key :type "Key Structure")))

(event `self.ReceiveTick`
  (params (DeltaSeconds :type "Float (single-precision)"))
  (bind _returnvalue (`HeadMountedDisplayFunctionLibrary.IsHeadMountedDisplayEnabled`))
  (bind _returnvalue_2 (`GameplayStatics.GetPlayerController` 0))
  (bind _returnvalue_3 (`KismetMathLibrary.Normal` (`KismetMathLibrary.ProjectVectorOnToPlane` (`SceneComponent.GetForwardVector` (`self.LeftMotionController`)) (0.0 0.0 1.0))))
  (`|ExecutionSequence`
    (:`then_0`
      ;[0.04384 0.4005 0.526] Movement
      (`self.AddMovementInput` (+ (* _returnvalue_3 (select `bool` _returnvalue :`false` (- (`KismetMathLibrary.Conv_BoolToDouble` (`PlayerController.IsInputKeyDown` _returnvalue_2 "S")) (`KismetMathLibrary.Conv_BoolToDouble` (`PlayerController.IsInputKeyDown` _returnvalue_2 "Z"))) :`true` (`self.GetInputAxisKeyValue`))) (* (`KismetMathLibrary.Cross_VectorVector` _returnvalue_3 (0.0 0.0 1.0)) (select `bool` _returnvalue :`false` (- (`KismetMathLibrary.Conv_BoolToDouble` (`PlayerController.IsInputKeyDown` _returnvalue_2 "D")) (`KismetMathLibrary.Conv_BoolToDouble` (`PlayerController.IsInputKeyDown` _returnvalue_2 "Q"))) :`true` (`self.GetInputAxisKeyValue`)))) -1.0))))

(event `Key|MouseScrollUp`
  (params (Key :type "Key Structure")))

(event `Key|LeftMouseButton`
  (params (Key :type "Key Structure")))

(event `Key|MotionController_Left_FaceButton2`
  (params (Key :type "Key Structure")))

(event `InputAxisKey|MouseX`
  (params (AxisValue :type "Float (single-precision)"))
  ;[0.04384 0.4005 0.526] Movement
  (if (not (`HeadMountedDisplayFunctionLibrary.IsHeadMountedDisplayEnabled`))
    (`self.AddControllerYawInput` AxisValue)))

(event `InputAxisKey|MouseY`
  (params (AxisValue :type "Float (single-precision)"))
  ;[0.04384 0.4005 0.526] Movement
  (if (not (`HeadMountedDisplayFunctionLibrary.IsHeadMountedDisplayEnabled`))
    (`self.AddControllerPitchInput` (* AxisValue -1.0))))

(event `Key|MotionController_Left_Grip1`
  (params (Key :type "Key Structure"))
  (bind _leftmotioncontroller (`self.LeftMotionController`))
  (bind _rightmotioncontroller (`self.RightMotionController`))
  ;[1 1 1] Grabbing
  (:`Pressed`
    (`self.GrabActor` (`self.LeftHandGrabSphere`) _leftmotioncontroller _rightmotioncontroller :!label _label))
  (:`Released`
    (`self.DropAll` _leftmotioncontroller _rightmotioncontroller :!label _label_2)))

(event `Key|MotionController_Left_Trigger`
  (params (Key :type "Key Structure"))
  ;[1 1 1] Grabbing
  (:`Pressed`
    (goto _label))
  (:`Released`
    (goto _label_2)))

(event `Key|MotionController_Right_Grip1`
  (params (Key :type "Key Structure"))
  (bind _rightmotioncontroller (`self.RightMotionController`))
  (bind _leftmotioncontroller (`self.LeftMotionController`))
  ;[1 1 1] Grabbing
  (:`Pressed`
    (`self.GrabActor` (`self.RightHandGrabSphere`) _rightmotioncontroller _leftmotioncontroller :!label _label_3))
  (:`Released`
    (`self.DropAll` _rightmotioncontroller _leftmotioncontroller :!label _label_4)))

(event `Key|MotionController_Right_Trigger`
  (params (Key :type "Key Structure"))
  ;[1 1 1] Grabbing
  (:`Pressed`
    (goto _label_3))
  (:`Released`
    (goto _label_4)))

(fn `DropAll`
  (params (MainHand :type "GripMotionControllerComponent Object Reference") (OtherHand :type "GripMotionControllerComponent Object Reference"))
  (bind _grippedactorsarray (`GripMotionControllerComponent.GetGrippedActors` MainHand))
  (for _array_element _grippedactorsarray
    (`GripMotionControllerComponent.DropActor` MainHand _array_element true (0.0 0.0 0.0) (0.0 0.0 0.0))
    (`SceneComponent.SetVisibility` MainHand true true)))

(fn `GrabActor`
  (params (SphereCollision :type "SphereComponent Object Reference") (MainHand :type "GripMotionControllerComponent Object Reference") (OtherHand :type "GripMotionControllerComponent Object Reference"))
  (bind _outactors (`KismetSystemLibrary.SphereOverlapActors` (`SceneComponent.K2_GetComponentLocation` SphereCollision) (`SphereComponent.SphereRadius` SphereCollision) (`|MakeArray` "ObjectTypeQuery7" :!type "EObjectTypeQuery Enum")))
  (for _array_element _outactors
    (if (`KismetSystemLibrary.DoesImplementInterface` _array_element "/Script/VRExpansionPlugin.VRGripInterface")
      (bind _grippedactorsarray (`GripMotionControllerComponent.GetGrippedActors` OtherHand))
      (bind _returnvalue (`self.GetOwner` _array_element))
      (bind _returnvalue_2 (select `bool` (`KismetSystemLibrary.DoesImplementInterface` _returnvalue "/Script/VRExpansionPlugin.VRGripInterface") :`false` _array_element :`true` _returnvalue))
      (if (`KismetArrayLibrary.Array_Contains` _grippedactorsarray _returnvalue_2)
        (`self.DropAll` OtherHand MainHand))
      (`GripMotionControllerComponent.GripActor` MainHand _returnvalue_2 (`self.GetTransform` _returnvalue_2) false "None" "InteractiveCollisionWithPhysics" "NotWhenCollidingOrDoubleGripping" "ForceClientSideMovement" 1500.0 200.0 false)
      (`SceneComponent.SetVisibility` MainHand false true)
      (break))))

(fn `UserConstructionScript`)