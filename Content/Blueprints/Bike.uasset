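; Bike actor that uses physics forces to keep its body upright, with stabilization switched on and off by Space or A.
; While enabled, each Tick projects the body's up vector onto its horizontal right axis to measure sideways lean.
; It applies a scaled opposing force at a point above the center of mass, creating a righting torque, and draws it as a debug arrow.
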(event `self.ReceiveBeginPlay`
  (`self.EnableInput` (`GameplayStatics.GetPlayerController` 0)))

(event `Key|SpaceBar`
  (params (Key :type "Key Structure"))
  (:`Pressed`
    (set `self.Stabilization` (not (`self.Stabilization`)) :!label _label)
    (`KismetSystemLibrary.PrintString` "SWITCH")))

(event `Key|A`
  (params (Key :type "Key Structure"))
  (:`Pressed`
    (goto _label)))

(event `self.ReceiveTick`
  (params (DeltaSeconds :type "Float (single-precision)"))
  (bind _bike_body (`self.Bike_Body`))
  (bind _returnvalue (+ (`PrimitiveComponent.GetCenterOfMass` _bike_body "None") (0.0 0.0 100.0)))
  (bind _returnvalue_2 (* (`KismetMathLibrary.ProjectVectorOnToVector` (`SceneComponent.GetUpVector` _bike_body) (`KismetMathLibrary.ProjectVectorOnToPlane` (`SceneComponent.GetRightVector` _bike_body) (0.0 0.0 1.0))) -100000.0))
  (if (`self.Stabilization`)
    (`PrimitiveComponent.AddForceAtLocation` _bike_body _returnvalue_2 _returnvalue "None")
    (`KismetSystemLibrary.DrawDebugArrow` _returnvalue (+ _returnvalue _returnvalue_2) 10.0 (struct :`R` 1.0 :`B` 0.565726 :`A` 1.0) 0.0 1.0)))

(fn `UserConstructionScript`)